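; Blue duck target for a shooting game whose BlueDuck component moves toward the height of the BpDuckEscape actor, re-issued every Tick.
; On overlap, a "Bullet" actor adds score and a round hit, while an "Escape" actor adds a miss; both destroy the duck.
; Both outcomes update per-round totals in bpGameInstance, advancing the round every two ducks and wrapping after five.
; Escape handling for rounds four and five is disconnected and never runs.
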(event EventBeginPlay)

(event Collision|EventActorBeginOverlap
  (params (OtherActor :type Actor%20Object%20Reference))
  (bind _returnvalue (Actor|ActorHasTag OtherActor "Escape"))
  ;[1 1 1] if true = bullet hit += to hit totals, if false = duck escape += miss totals. Both contribute to round totals
  (if (Actor|ActorHasTag OtherActor "Bullet")
    (bind _asbp_game_instance (Utilities|Casting|CastTobpGameInstance (Game|GetGameInstance)))
    (Variables|/Game/BluePrints/bpGameInstance.bpGameInstance_C|SetScore _asbp_game_instance (+ (Variables|/Game/BluePrints/bpGameInstance.bpGameInstance_C|GetScore _asbp_game_instance) 1000))
    (Actor|DestroyActor)
    (bind _asbp_game_instance_2 (Utilities|Casting|CastTobpGameInstance (Game|GetGameInstance)))
    (if (== (Variables|/Game/BluePrints/bpGameInstance.bpGameInstance_C|GetRound _asbp_game_instance_2) 1)
      (bind _asbp_game_instance_3 (Utilities|Casting|CastTobpGameInstance (Game|GetGameInstance)))
      (Variables|/Game/BluePrints/bpGameInstance.bpGameInstance_C|SetRoundOneHit _asbp_game_instance_3 (+ (Variables|/Game/BluePrints/bpGameInstance.bpGameInstance_C|GetRoundOneHit _asbp_game_instance_3) 1))
      (bind _asbp_game_instance_4 (Utilities|Casting|CastTobpGameInstance (Game|GetGameInstance)))
      (Variables|/Game/BluePrints/bpGameInstance.bpGameInstance_C|SetRoundOneTotal _asbp_game_instance_4 (+ (Variables|/Game/BluePrints/bpGameInstance.bpGameInstance_C|GetRoundOneTotal _asbp_game_instance_4) 1))
      (bind _asbp_game_instance_5 (Utilities|Casting|CastTobpGameInstance (Game|GetGameInstance)))
      (if (== (Variables|/Game/BluePrints/bpGameInstance.bpGameInstance_C|GetRoundOneTotal _asbp_game_instance_5) 2)
        (Variables|/Game/BluePrints/bpGameInstance.bpGameInstance_C|SetRound _asbp_game_instance_5 2))
      (elif (== (Variables|/Game/BluePrints/bpGameInstance.bpGameInstance_C|GetRound _asbp_game_instance_2) 2)
        (bind _asbp_game_instance_6 (Utilities|Casting|CastTobpGameInstance (Game|GetGameInstance)))
        (Variables|/Game/BluePrints/bpGameInstance.bpGameInstance_C|SetRoundTwoHit _asbp_game_instance_6 (+ (Variables|/Game/BluePrints/bpGameInstance.bpGameInstance_C|GetRoundTwoHit _asbp_game_instance_6) 1))
        (bind _asbp_game_instance_7 (Utilities|Casting|CastTobpGameInstance (Game|GetGameInstance)))
        (Variables|/Game/BluePrints/bpGameInstance.bpGameInstance_C|SetRoundTwoTotal _asbp_game_instance_7 (+ (Variables|/Game/BluePrints/bpGameInstance.bpGameInstance_C|GetRoundTwoTotal _asbp_game_instance_7) 1))
        (bind _asbp_game_instance_8 (Utilities|Casting|CastTobpGameInstance (Game|GetGameInstance)))
        (if (== (Variables|/Game/BluePrints/bpGameInstance.bpGameInstance_C|GetRoundTwoTotal _asbp_game_instance_8) 2)
          (Variables|/Game/BluePrints/bpGameInstance.bpGameInstance_C|SetRound _asbp_game_instance_8 3))
        (elif (== (Variables|/Game/BluePrints/bpGameInstance.bpGameInstance_C|GetRound _asbp_game_instance_2) 3)
          (bind _asbp_game_instance_9 (Utilities|Casting|CastTobpGameInstance (Game|GetGameInstance)))
          (Variables|/Game/BluePrints/bpGameInstance.bpGameInstance_C|SetRoundThreeHit _asbp_game_instance_9 (+ (Variables|/Game/BluePrints/bpGameInstance.bpGameInstance_C|GetRoundThreeHit _asbp_game_instance_9) 1))
          (bind _asbp_game_instance_10 (Utilities|Casting|CastTobpGameInstance (Game|GetGameInstance)))
          (Variables|/Game/BluePrints/bpGameInstance.bpGameInstance_C|SetRoundThreeTotal _asbp_game_instance_10 (+ (Variables|/Game/BluePrints/bpGameInstance.bpGameInstance_C|GetRoundThreeTotal _asbp_game_instance_10) 1))
          (bind _asbp_game_instance_11 (Utilities|Casting|CastTobpGameInstance (Game|GetGameInstance)))
          (if (== (Variables|/Game/BluePrints/bpGameInstance.bpGameInstance_C|GetRoundThreeTotal _asbp_game_instance_11) 2)
            (Variables|/Game/BluePrints/bpGameInstance.bpGameInstance_C|SetRound _asbp_game_instance_11 4))
          (elif (== (Variables|/Game/BluePrints/bpGameInstance.bpGameInstance_C|GetRound _asbp_game_instance_2) 4)
            (bind _asbp_game_instance_12 (Utilities|Casting|CastTobpGameInstance (Game|GetGameInstance)))
            (Variables|/Game/BluePrints/bpGameInstance.bpGameInstance_C|SetRoundFourHit _asbp_game_instance_12 (+ (Variables|/Game/BluePrints/bpGameInstance.bpGameInstance_C|GetRoundFourHit _asbp_game_instance_12) 1))
            (bind _asbp_game_instance_13 (Utilities|Casting|CastTobpGameInstance (Game|GetGameInstance)))
            (Variables|/Game/BluePrints/bpGameInstance.bpGameInstance_C|SetRoundFourTotal _asbp_game_instance_13 (+ (Variables|/Game/BluePrints/bpGameInstance.bpGameInstance_C|GetRoundFourTotal _asbp_game_instance_13) 1))
            (bind _asbp_game_instance_14 (Utilities|Casting|CastTobpGameInstance (Game|GetGameInstance)))
            (if (== (Variables|/Game/BluePrints/bpGameInstance.bpGameInstance_C|GetRoundFourTotal _asbp_game_instance_14) 2)
              (Variables|/Game/BluePrints/bpGameInstance.bpGameInstance_C|SetRound _asbp_game_instance_14 5))
            (elif (== (Variables|/Game/BluePrints/bpGameInstance.bpGameInstance_C|GetRound _asbp_game_instance_2) 5)
              (bind _asbp_game_instance_15 (Utilities|Casting|CastTobpGameInstance (Game|GetGameInstance)))
              (Variables|/Game/BluePrints/bpGameInstance.bpGameInstance_C|SetRoundFiveHit _asbp_game_instance_15 (+ (Variables|/Game/BluePrints/bpGameInstance.bpGameInstance_C|GetRoundFiveHit _asbp_game_instance_15) 1))
              (bind _asbp_game_instance_16 (Utilities|Casting|CastTobpGameInstance (Game|GetGameInstance)))
              (Variables|/Game/BluePrints/bpGameInstance.bpGameInstance_C|SetRoundFiveTotal _asbp_game_instance_16 (+ (Variables|/Game/BluePrints/bpGameInstance.bpGameInstance_C|GetRoundFiveTotal _asbp_game_instance_16) 1))
              (bind _asbp_game_instance_17 (Utilities|Casting|CastTobpGameInstance (Game|GetGameInstance)))
              (if (== (Variables|/Game/BluePrints/bpGameInstance.bpGameInstance_C|GetRoundFiveTotal _asbp_game_instance_17) 2)
                (Variables|/Game/BluePrints/bpGameInstance.bpGameInstance_C|SetRound _asbp_game_instance_17 1)))))))
    (else
      (bind _asbp_game_instance_18 (Utilities|Casting|CastTobpGameInstance (Game|GetGameInstance)))
      (if (and (== (Variables|/Game/BluePrints/bpGameInstance.bpGameInstance_C|GetRound _asbp_game_instance_18) 1) _returnvalue)
        (Actor|DestroyActor)
        (bind _asbp_game_instance_19 (Utilities|Casting|CastTobpGameInstance (Game|GetGameInstance)))
        (Variables|/Game/BluePrints/bpGameInstance.bpGameInstance_C|SetRoundOneTotal _asbp_game_instance_19 (+ (Variables|/Game/BluePrints/bpGameInstance.bpGameInstance_C|GetRoundOneTotal _asbp_game_instance_19) 1))
        (bind _asbp_game_instance_20 (Utilities|Casting|CastTobpGameInstance (Game|GetGameInstance)))
        (Variables|/Game/BluePrints/bpGameInstance.bpGameInstance_C|SetTotalMissed _asbp_game_instance_20 (+ (Variables|/Game/BluePrints/bpGameInstance.bpGameInstance_C|GetTotalMissed _asbp_game_instance_20) 1))
        (bind _asbp_game_instance_21 (Utilities|Casting|CastTobpGameInstance (Game|GetGameInstance)))
        (if (== (Variables|/Game/BluePrints/bpGameInstance.bpGameInstance_C|GetRoundOneTotal _asbp_game_instance_21) 2)
          (Variables|/Game/BluePrints/bpGameInstance.bpGameInstance_C|SetRound _asbp_game_instance_21 2))
        (elif (and (== (Variables|/Game/BluePrints/bpGameInstance.bpGameInstance_C|GetRound _asbp_game_instance_18) 2) _returnvalue)
          (Actor|DestroyActor)
          (bind _asbp_game_instance_22 (Utilities|Casting|CastTobpGameInstance (Game|GetGameInstance)))
          (Variables|/Game/BluePrints/bpGameInstance.bpGameInstance_C|SetRoundTwoTotal _asbp_game_instance_22 (+ (Variables|/Game/BluePrints/bpGameInstance.bpGameInstance_C|GetRoundTwoTotal _asbp_game_instance_22) 1))
          (bind _asbp_game_instance_23 (Utilities|Casting|CastTobpGameInstance (Game|GetGameInstance)))
          (Variables|/Game/BluePrints/bpGameInstance.bpGameInstance_C|SetTotalMissed _asbp_game_instance_23 (+ (Variables|/Game/BluePrints/bpGameInstance.bpGameInstance_C|GetTotalMissed _asbp_game_instance_23) 1))
          (bind _asbp_game_instance_24 (Utilities|Casting|CastTobpGameInstance (Game|GetGameInstance)))
          (if (== (Variables|/Game/BluePrints/bpGameInstance.bpGameInstance_C|GetRoundTwoTotal _asbp_game_instance_24) 2)
            (Variables|/Game/BluePrints/bpGameInstance.bpGameInstance_C|SetRound _asbp_game_instance_24 3))
          (elif (and (== (Variables|/Game/BluePrints/bpGameInstance.bpGameInstance_C|GetRound _asbp_game_instance_18) 3) _returnvalue)
            (Actor|DestroyActor)
            (bind _asbp_game_instance_25 (Utilities|Casting|CastTobpGameInstance (Game|GetGameInstance)))
            (Variables|/Game/BluePrints/bpGameInstance.bpGameInstance_C|SetRoundThreeTotal _asbp_game_instance_25 (+ (Variables|/Game/BluePrints/bpGameInstance.bpGameInstance_C|GetRoundThreeTotal _asbp_game_instance_25) 1))
            (bind _asbp_game_instance_26 (Utilities|Casting|CastTobpGameInstance (Game|GetGameInstance)))
            (Variables|/Game/BluePrints/bpGameInstance.bpGameInstance_C|SetTotalMissed _asbp_game_instance_26 (+ (Variables|/Game/BluePrints/bpGameInstance.bpGameInstance_C|GetTotalMissed _asbp_game_instance_26) 1))
            (bind _asbp_game_instance_27 (Utilities|Casting|CastTobpGameInstance (Game|GetGameInstance)))
            (if (== (Variables|/Game/BluePrints/bpGameInstance.bpGameInstance_C|GetRoundThreeTotal _asbp_game_instance_27) 2)
              (Variables|/Game/BluePrints/bpGameInstance.bpGameInstance_C|SetRound _asbp_game_instance_27 4))))))))

(event EventTick
  (params (DeltaSeconds :type Float%20%28single-precision%29))
  (bind _returnvalue (Actor|GetActorOfClass "/Game/BluePrints/bpDuckEscape.bpDuckEscape_C"))
  (if (!= _returnvalue 0)
    (Components|MoveComponentTo (Variables|Default|GetBlueDuck) (Math|Vector|MakeVector 0.0 0.0 (.z (Transformation|GetActorLocation _returnvalue))) "0, 0, 0" false false (Variables|Default|GetMoveTime) false)))

(fn ConstructionScript)